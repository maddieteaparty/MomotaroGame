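; Base player character Blueprint that handles two combo attacks, temporary hitboxes and hostile hit detection.
; Attack events from the Player Controller interface drive an attack state and per-attack counters; timers restore idle and clear lapsed combos, with a longer third hit.
; SpawnHitbox adds a timed overlap box, but its damage input is unused.
; Attacks and tag-checked HurtBox overlaps only print debug text; construction sets walk speed.
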(event `/Game/_Input/BI_Attack1.Attack1`
  (bind _attackrate_a1 (`self.attackRate_A1`))
  (bind _attackcombocounter_a1 (`self.attackComboCounter_A1`))
  ;[1 1 1] Attack 1
  (if (`|EnumEquality` (`self.attackState`) "NewEnumerator0")
    (set `self.attackState` "NewEnumerator1" :!label _label)
    (`/Engine/EditorBlueprintResources/StandardMacros.IncrementInt` _attackcombocounter_a1
      (:`  `
        (if (>= _attackcombocounter_a1 3)
          ;;[1 1 1] Final Hit
          (`KismetSystemLibrary.PrintString` "Attack 1 Final Hit")
          (`KismetSystemLibrary.K2_SetTimerDelegate` (delegate `ResetAttackState`) (* (`self.attackRate_A1`) 2.0)) ; Set to idle after attack is done.
          (else
            ;;[1 1 1] Basic Hit
            (`KismetSystemLibrary.PrintString` "Attack 1 Hit")
            (`KismetSystemLibrary.K2_SetTimerDelegate` (delegate `ResetAttackState`) (`self.attackRate_A1`)) ; Set to idle after attack is done.
          ))
        (`KismetSystemLibrary.K2_SetTimerDelegate` (delegate `Attack1ComboCheck`) (+ _attackrate_a1 (/ _attackrate_a1 2.0))) ; Check to see if player is continuing combo.
      ))
    (elif (`self.attackContinueCheck_A1`)
      (set `self.attackContinueCheck_A1` false)
      (goto _label))))

(event `Attack1ComboCheck`
  ;[1 1 1] Attack 1
  ;;[1 1 1] Attack 1 Combo Check
  (if (not (`|EnumEquality` (`self.attackState`) "NewEnumerator1"))
    (set `self.attackComboCounter_A1` 0)))

(event `ResetAttackState`
  ;[1 1 1] Reset to Idle After Attack
  (set `self.attackState` "NewEnumerator0")
  (if (>= (`self.attackComboCounter_A1`) 3)
    (set `self.attackComboCounter_A1` 0))
  (if (>= (`self.attackComboCounter_A2`) 3)
    (set `self.attackComboCounter_A2` 0)))

(event `/Game/_Input/BI_Attack2.Attack2`
  (bind _attackrate_a2 (`self.attackRate_A2`))
  (bind _attackcombocounter_a2 (`self.attackComboCounter_A2`))
  ;[1 1 1] Attack 2
  (if (`|EnumEquality` (`self.attackState`) "NewEnumerator0")
    (set `self.attackState` "NewEnumerator2")
    (`/Engine/EditorBlueprintResources/StandardMacros.IncrementInt` _attackcombocounter_a2
      (:`  `
        (if (>= _attackcombocounter_a2 3)
          ;;[1 1 1] Final Hit
          (`KismetSystemLibrary.PrintString` "Attack 2 Final Hit")
          (`KismetSystemLibrary.K2_SetTimerDelegate` (delegate `ResetAttackState`) (* (`self.attackRate_A2`) 2.0)) ; Set to idle after attack is done.
          (else
            ;;[1 1 1] Basic Hit
            (`KismetSystemLibrary.PrintString` "Attack 2 Hit")
            (`KismetSystemLibrary.K2_SetTimerDelegate` (delegate `ResetAttackState`) (`self.attackRate_A2`)) ; Set to idle after attack is done.
          ))
        (`KismetSystemLibrary.K2_SetTimerDelegate` (delegate `Attack2CombCheck`) (+ _attackrate_a2 (/ _attackrate_a2 2.0))) ; Check to see if player is continuing combo.
      ))))

(event `Attack2CombCheck`
  ;[1 1 1] Attack 2
  ;;[1 1 1] Attack 1 Combo Check
  (if (not (`|EnumEquality` (`self.attackState`) "NewEnumerator2"))
    (set `self.attackComboCounter_A2` 0)))

(event `SpawnHitbox`
  (params (RelativeTransform :type "Transform Structure") (`Hitbox Lifetime` :type "Float (double-precision)") (`Hitbox Damage` :type "Float (double-precision)"))
  (bind _returnvalue (`|AddComponentByClass` "/Script/Engine.BoxComponent" false RelativeTransform))
  (`PrimitiveComponent.SetCollisionResponseToAllChannels` _returnvalue "ECR_Overlap")
  (`KismetSystemLibrary.Delay` `Hitbox Lifetime`)
  (`ActorComponent.K2_DestroyComponent` _returnvalue))

(event `self.HurtBox.OnComponentBeginOverlap`
  (params (OverlappedComponent :type "PrimitiveComponent Object Reference") (OtherActor :type "Actor Object Reference") (OtherComp :type "PrimitiveComponent Object Reference") (OtherBodyIndex :type Integer) (bFromSweep :type Boolean) (SweepResult :type "HitResult Structure (by ref)"))
  ;[1 1 1] Take Damage
  (if (`ActorComponent.ComponentHasTag` OtherComp (`self.HitboxTagName`))
    (`KismetSystemLibrary.PrintString` "overlapping hostile hitbox!")))

(fn `UserConstructionScript`
  (set `CharacterMovementComponent.MaxWalkSpeed` (`self.walkSpeed`) (`self.CharacterMovement`)))